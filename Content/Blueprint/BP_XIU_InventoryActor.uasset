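; BP_XIU_InventoryActor is an item actor in the world that can be picked up by overlapping it.
; On overlap, the authority gets the inventory component through XIUInventoryInterface on the other actor and passes it to TryPickUp.
; When its own inventory component fires the server change delegate, it sets its static mesh from the held BP_XIU_BaseItem, or clears it if that cast fails.
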(event `self.ReceiveActorBeginOverlap`
  (params (OtherActor :type "Actor Object Reference"))
  (`/Engine/EditorBlueprintResources/ActorMacros.Switch Has Authority`
    (:`Authority`
      (bind _asxiuinventory_interface (cast `XIUInventoryInterface` OtherActor))
      (bind _returnvalue (`XIUInventoryInterface.GetInventoryComponent` _asxiuinventory_interface))
      (`XIUPickUpInterface.TryPickUp` _returnvalue))))

(event `self.InventoryComponent.InventoryChangedServerDelegate`
  (`self.UpdateStaticMesh`))

(fn `UpdateStaticMesh`
  (bind _returnvalue (`XIUPickUpInterface.GetItem`))
  (bind _asbp_xiu_base_item (cast `/XyloInventoryUtil/Blueprint/Item/BP_XIU_BaseItem` _returnvalue)
    (:`then`
      (bind _itemmesh (`/XyloInventoryUtil/Blueprint/Item/BP_XIU_BaseItem.GetItemMesh` _asbp_xiu_base_item))
      (`StaticMeshComponent.SetStaticMesh` (`self.StaticMesh`) _itemmesh))
    (:`CastFailed`
      (`StaticMeshComponent.SetStaticMesh` (`self.StaticMesh`) null))))

(fn `UserConstructionScript`)