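; BP_XIU_ItemActor is a world item pickup that transfers its Item into an inventory when an actor overlaps it.
; On the authority, it gets the inventory component from overlapping actors implementing XIUInventoryInterface and adds the Item.
; It destroys itself if the Item is invalid or emptied, otherwise refreshes its mesh for the remainder.
; ItemSet also refreshes the static mesh, which comes from the Item and is cleared when empty.
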(event `self.ReceiveActorBeginOverlap`
  (params (OtherActor :type "Actor Object Reference"))
  (`/Engine/EditorBlueprintResources/ActorMacros.Switch Has Authority`
    (:`Authority`
      (bind _asxiuinventory_interface (cast `XIUInventoryInterface` OtherActor))
      (bind _returnvalue (`XIUInventoryInterface.GetInventoryComponent` _asxiuinventory_interface))
      (`/Engine/EditorBlueprintResources/StandardMacros.IsValid` (`self.Item`)
        (:`Is Valid`
          (`XIUInventoryComponent.AddItem` _returnvalue (`self.Item`))
          (if (`XIUItem.IsEmpty` (`self.Item`))
            (`self.K2_DestroyActor`)
            (else
              (`self.UpdateStaticMesh`))))
        (:`Is Not Valid`
          (`self.K2_DestroyActor`))))))

(event `self.BP_ItemSet`
  (`self.UpdateStaticMesh`))

(fn `UpdateStaticMesh`
  (`/Engine/EditorBlueprintResources/StandardMacros.IsValid` (`self.Item`)
    (:`Is Valid`
      (if (`XIUItem.IsEmpty` (`self.Item`))
        (`StaticMeshComponent.SetStaticMesh` (`self.StaticMesh`) null)
        (else
          (`StaticMeshComponent.SetStaticMesh` (`self.StaticMesh`) (`XIUItem.GetItemMesh` (`self.Item`))))))))

(fn `UserConstructionScript`)